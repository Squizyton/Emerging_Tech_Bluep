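; Overlap-driven button actor that signals an on or off state as actors enter and leave it.
; Begin and end overlap set the IntTrigger flag and share one branch, which calls ButtonTrue or ButtonFalse, apparently event dispatchers for other Blueprints to bind.
; Each event also flips the TextRender's visibility, with no filter on the overlapping actor or count of simultaneous overlaps.
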(event Collision|EventActorBeginOverlap
  (params (OtherActor :type Actor%20Object%20Reference))
  (Variables|Default|SetintTrigger true)
  (if (Variables|Default|GetintTrigger)
    (Rendering|ToggleVisibility (Variables|Default|GetTextRender) false)
    (Default|CallButtonTrue)
    (else
      (Rendering|ToggleVisibility (Variables|Default|GetTextRender) false)
      (Default|CallButtonFalse))))

(event Collision|EventActorEndOverlap
  (params (OtherActor :type Actor%20Object%20Reference))
  (Variables|Default|SetintTrigger false)
  (if (Variables|Default|GetintTrigger)
    (Rendering|ToggleVisibility (Variables|Default|GetTextRender) false)
    (Default|CallButtonTrue)
    (else
      (Rendering|ToggleVisibility (Variables|Default|GetTextRender) false)
      (Default|CallButtonFalse))))

(fn ConstructionScript)